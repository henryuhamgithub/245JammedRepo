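; BP_FallingObject is a falling hazard actor that damages the third-person character on contact.
; Its Box overlap applies fixed damage only while HasCollided is false, then sets that flag so damage happens once.
; A hit on the Cube also sets the flag, so the object is harmless after striking something.
; BeginPlay clears the flag, adds a static mesh component at an offset, and prints a debug message after a short delay.
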(event `self.Box.OnComponentBeginOverlap`
  (params (OverlappedComponent :type "PrimitiveComponent Object Reference") (OtherActor :type "Actor Object Reference") (OtherComp :type "PrimitiveComponent Object Reference") (OtherBodyIndex :type Integer) (bFromSweep :type Boolean) (SweepResult :type "HitResult Structure (by ref)"))
  (bind _asbp_third_person_character (cast `/Game/ThirdPerson/Blueprints/BP_ThirdPersonCharacter` OtherActor))
  (if (`self.hasCollided`)
    (set `self.hasCollided` true)
    (else
      (set `self.hasCollided` true)
      (`GameplayStatics.ApplyDamage` _asbp_third_person_character 34.0))))

(event `self.Cube.OnComponentHit`
  (params (HitComponent :type "PrimitiveComponent Object Reference") (OtherActor :type "Actor Object Reference") (OtherComp :type "PrimitiveComponent Object Reference") (NormalImpulse :type "Vector Structure") (Hit :type "HitResult Structure (by ref)"))
  (set `self.hasCollided` true))

(event `self.ReceiveBeginPlay`
  (set `self.hasCollided` false)
  (`AddComponent|NODE_AddStaticMeshComponent-0` :`RelativeTransform` (`KismetMathLibrary.MakeTransform` (370.0 70.0 1.0)))
  (`KismetSystemLibrary.Delay` 0.3)
  (`KismetSystemLibrary.PrintString` "Hello"))

(fn `UserConstructionScript`)